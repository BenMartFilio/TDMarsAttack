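; BP_Joueur is the player pawn, a side-scrolling camera that also spawns human units.
; BeginPlay adds the IMC_Camera Enhanced Input context, but only when the controller is a PC_MenuStart.
; IA_Camera moves the pawn along the camera's right vector.
; Hard-bound Space and E keys both call SpawnHumain, which spawns BP_UniteHumaine01 as AI with no location wired, though its comment intends the base.
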(event `EnhancedInput|/Game/Inputs/IA_Camera`
  (params (ActionValue :type "Float (double-precision)") (ElapsedSeconds :type "Float (double-precision)") (TriggeredSeconds :type "Float (double-precision)") (InputAction :type "InputAction Object Reference" :default "/Game/Inputs/IA_Camera.IA_Camera"))
  ; Mouvement de la caméra
  (:`Triggered`
    (`self.AddMovementInput` self (`SceneComponent.GetRightVector` (`self.Camera`)) ActionValue false)))

(event `Key|SpaceBar`
  (params (Key :type "Key Structure"))
  (:`Pressed`
    (`self.SpawnHumain` :!label _label)))

(event `Key|E`
  (params (Key :type "Key Structure"))
  (:`Pressed`
    (goto _label)))

(event `SpawnHumain`
  ; Fait spawner les unités à l'emplacement de la base
  (`AIBlueprintHelperLibrary.SpawnAIFromClass` "/Game/Blueprint/Elements/Unite/BP_UniteHumaine01.BP_UniteHumaine01_C" null (0.0 0.0 0.0) (struct) false null))

(event `self.ReceiveBeginPlay`
  ; A faire enhanced inpu local subsystem
  (bind _aspc_menu_start (cast `/Game/Blueprint/PlayerController/PC_MenuStart` (`self.GetController`)))
  (`EnhancedInputSubsystemInterface.AddMappingContext` (pcsubsystem `EnhancedInputLocalPlayerSubsystem` _aspc_menu_start) "/Game/Inputs/IMC_Camera.IMC_Camera" 0 (struct)))

(fn `UserConstructionScript`)