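; Start-menu PlayerController that shows HUD_MenuStart with a visible cursor and handles multiplayer hosting and joining.
; Hosting creates a session with two public connections, then opens MapPrincipale as a listen server.
; Searching refills the menu's session list with one HUD_Sessions widget per result, whose button triggers JoinSession.
; Direct IP connection runs an "open" console command, appending the IP without a separating space.
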(event `JoinSession`
  (params (SearchResult :type "BlueprintSessionResult Structure (by ref)"))
  ; Rejoins la session lorsqu'on clique sur le bouton qui lui est associé (dans hud_sessions)
  (`JoinSessionCallbackProxy.JoinSession` self SearchResult))

(event `Rechercher`
  ; Recherche les sessions disponible sur votre LAN
  (`PanelWidget.ClearChildren` (`/Game/HUD/HUD_MenuStart.EmplacementSessions` (`self.HUD_MenuStart`)))
  (set `self.IsFindingSession` true)
  (bind _results (`FindSessionsCallbackProxy.FindSessions` self 6) ; Ajouter au On Failure la fin du chargement et un message pas de sessions trouvées
    (:`OnSuccess`
      (for _array_element _results
        (bind _returnvalue (`|CreateWidget` "/Game/HUD/HUD_Sessions.HUD_Sessions_C" null _array_element))
        (`PanelWidget.AddChild` (`/Game/HUD/HUD_MenuStart.EmplacementSessions` (`self.HUD_MenuStart`)) _returnvalue))
      (set `self.IsFindingSession` false))))

(event `self.ReceiveBeginPlay`
  ; Ce qu'il se passe lorsque le jeu se lance
  (`self.Menu HUD`)
  (`self.Show Cursor`))

(event `Hebergement`
  ;[1 0.07292 0.07292 0.5] Permet d'héberger la session
  (`CreateSessionCallbackProxy.CreateSession` self 2
    (:`OnSuccess`
      (`GameplayStatics.OpenLevelBySoftObjectPtr` "/Game/Map/MapPrincipale.MapPrincipale" true "listen"))))

(event `Show Cursor`
  ; Afficher le curseur
  (set `self.bShowMouseCursor` true)
  (`WidgetBlueprintLibrary.SetInputMode_GameAndUIEx` self null "LockAlways" false))

(event `Connexion`
  (params (IP :type String))
  ;[0.8698 0.06795 0.06795 0.5] Permet de te connecter lorsque tu rentres une ip
  (`KismetSystemLibrary.ExecuteConsoleCommand` (`KismetStringLibrary.Concat_StrStr` "open " IP) null))

(event `Menu HUD`
  ; Création du menu de base
  (`/Engine/EditorBlueprintResources/StandardMacros.IsValid` (`self.HUD_MenuStart`)
    (:`Is Not Valid`
      (bind _returnvalue (`|CreateWidget` "/Game/HUD/HUD_MenuStart.HUD_MenuStart_C"))
      (bind _output_get (set `self.HUD_MenuStart` _returnvalue))
      (`UserWidget.AddToViewport` _output_get 0))))

(fn `UserConstructionScript`)