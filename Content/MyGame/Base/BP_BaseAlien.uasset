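; BP_BaseAlien is the alien base actor, which has health and is destroyed when it reaches zero.
; On BeginPlay it creates a WBP_BaseAlienHp1 health bar, initializes it with MaxHealth and adds it to the viewport.
; HpSystemBase subtracts incoming human damage, clamps health between zero and max, updates the widget, and calls DeathBase at zero to destroy the actor.
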(event `self.ReceiveBeginPlay`
  (`self.CreationAlienne`))

(event `CreationAlienne`
  ; Creation widget barre de vie, et récupère hp
  (bind _returnvalue (`|CreateWidget` "/Game/MyGame/Widget/WBP_BaseAlienHp1.WBP_BaseAlienHp1_C"))
  (bind _output_get (set `self.HealthBarRef` _returnvalue))
  (set `/Game/MyGame/Widget/WBP_BaseAlienHp1.HealthWidget` (`self.MaxHealth`) _output_get)
  (`UserWidget.AddToViewport` _output_get 0))

(event `HpSystemBase`
  (params (Damage :type "Float (double-precision)"))
  ; Degat quand elle se fait toucher
  (set `self.HumanDamage` Damage)
  (bind _output_get (set `self.Health` (`KismetMathLibrary.FClamp` (- (`self.Health`) (`self.HumanDamage`)) 0.0 (`self.MaxHealth`))))
  (set `/Game/MyGame/Widget/WBP_BaseAlienHp1.HealthWidget` _output_get (`self.HealthBarRef`))
  ; Vérifie si base toujours en vie
  (if (== (`self.Health`) 0.0)
    (`self.DeathBase`)))

(event `DeathBase`
  (`self.K2_DestroyActor`))

(fn `UserConstructionScript`)