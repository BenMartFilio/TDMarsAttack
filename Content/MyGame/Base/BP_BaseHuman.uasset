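; Human base actor with health that is destroyed when that health reaches zero.
; On BeginPlay it creates a health widget, seeds it with max health and adds it to the viewport.
; A health event subtracts damage with clamping, updates the widget and triggers destruction at zero.
; AnyDamage calls that event with a fixed zero instead of passing the received damage.
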(event `self.ReceiveBeginPlay`
  (`self.CreationHumaine`))

(event `CreationHumaine`
  (bind _returnvalue (`|CreateWidget` "/Game/MyGame/Widget/WBP_BaseHumanHp.WBP_BaseHumanHp_C" null null))
  (bind _output_get (set `self.HealthBarRef` _returnvalue))
  (set `/Game/MyGame/Widget/WBP_BaseHumanHp.HealthWidget` (`self.MaxHealth`) _output_get)
  (`UserWidget.AddToViewport` _output_get 0))

(event `self.ReceiveAnyDamage`
  (params (Damage :type "Float (single-precision)") (DamageType :type "DamageType Object Reference") (InstigatedBy :type "Controller Object Reference") (DamageCauser :type "Actor Object Reference"))
  (set `self.Damage` Damage)
  (`self.HpSystemBase` 0.0))

(event `HpSystemBase`
  (params (Damage :type "Float (double-precision)"))
  (set `self.Damage` Damage)
  (bind _output_get (set `self.Health` (`KismetMathLibrary.FClamp` (- (`self.Health`) (`self.Damage`)) 0.0 (`self.MaxHealth`))))
  (set `/Game/MyGame/Widget/WBP_BaseHumanHp.HealthWidget` _output_get (`self.HealthBarRef`))
  ; Vérifie si base toujours en vie
  (if (== (`self.Health`) 0.0)
    (`self.DeathBase`)))

(event `DeathBase`
  (`self.K2_DestroyActor`))

(fn `UserConstructionScript`)