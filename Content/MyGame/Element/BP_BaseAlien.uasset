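; BP_BaseAlien is a damageable alien base actor that destroys itself when its health reaches zero.
; On BeginPlay it creates a WBP_BaseAlienHp1 health bar, adds it to the viewport and fills it with MaxHealth.
; AnyDamage and HpSystemBase share logic that subtracts damage from clamped Health and calls DeathBase at zero.
; That logic writes MaxHealth to the bar instead of current Health.
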(event `self.ReceiveBeginPlay`
  (bind _returnvalue (`|CreateWidget` "/Game/MyGame/Widget/WBP_BaseAlienHp1.WBP_BaseAlienHp1_C"))
  (bind _output_get (set `self.HealthBarRef` _returnvalue))
  (`UserWidget.AddToViewport` _output_get 0)
  (set `/Game/MyGame/Widget/WBP_BaseAlienHp1.Health` (`self.MaxHealth`) _output_get))

(event `HpSystemBase`
  (set `self.Health` (`KismetMathLibrary.FClamp` (- (`self.Health`) (stale `self.ReceiveAnyDamage` Damage)) 0.0 (`self.MaxHealth`)) :!label _label)
  (set `/Game/MyGame/Widget/WBP_BaseAlienHp1.Health` (`self.MaxHealth`) (`self.HealthBarRef`))
  ; Vérifie si base toujours en vie
  (if (== (`self.Health`) 0.0)
    (`self.DeathBase`)))

(event `self.ReceiveAnyDamage`
  (params (Damage :type "Float (single-precision)") (DamageType :type "DamageType Object Reference") (InstigatedBy :type "Controller Object Reference") (DamageCauser :type "Actor Object Reference"))
  (goto _label))

(event `DeathBase`
  (`self.K2_DestroyActor`))

(fn `UserConstructionScript`)